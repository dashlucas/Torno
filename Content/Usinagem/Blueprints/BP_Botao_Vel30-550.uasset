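; BP_Botao_Vel30-550 is a draggable speed control for the 30-550 range in the Usinagem (machining) module.
; Drag updates from Comp_Drag store distance, percent and velocity, then pass only the percent to RefConfigsGerais.ComVelocidades30550, with velocity and distance zeroed.
; The same percent drives a Pitch event that raises the sound pitch on the referenced chuck-jaw power button (RefBotaoLigarCastanhas) by linear interpolation.
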(event DragStateChangedConstant(Comp_Drag)
  (params (Name :type Name :default "None") (Distance :type Float%20%28single-precision%29) (Procent :type Float%20%28single-precision%29) (Velocity :type Float%20%28single-precision%29) (Source :type Actor%20Object%20Reference) (Pawn :type BP%20Pawn%20Base%20Object%20Reference))
  (Variables|Default|SetDistance Distance)
  (Variables|Default|SetProcent Procent)
  (Variables|Default|SetVelocity Velocity)
  (Default|ComVelocidades30-550 (Variables|Default|GetRef_Configs_Gerais) 0.0 (Variables|Default|GetProcent) 0.0)
  (CallFunction|Pitch))

(event Custom|Pitch
  ;[1 1 1] Mudar Pitch
  (Audio|Components|Audio|SetPitchMultiplier (Variables|/Game/Usinagem/Blueprints/BP_BotaoLigar_Castanhas.BP_BotaoLigar_Castanhas_C|GetSom (Variables|Default|GetRef_BotaoLigar_Castanhas)) (Math|Float|Lerp 1.0 1.5 (Variables|Default|GetProcent))))

(event EventBeginPlay)

(event Collision|EventActorBeginOverlap
  (params (OtherActor :type Actor%20Object%20Reference)))

(fn ConstructionScript)