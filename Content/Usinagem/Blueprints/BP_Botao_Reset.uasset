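; BP_Botao_Reset is the reset button in a machining (Usinagem) scene.
; Its drag component's state-change event sets ResetLigado true only when the section is set and the general config's PodeApertarReset allows pressing.
; On success it calls LigarOGiroDasCastanhas on the warnings reference (RefAvisos).
; Otherwise it clears the flag and triggers either the loose-guard warning when power is on or the main-switch warning when it is off.
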(event DragStateChangedSingle(Comp_Drag)
  (params (Identifier :type Name :default "None") (Section :type Struct%20Section%20Structure) (Source :type Actor%20Object%20Reference) (Pawn :type BP%20Pawn%20Base%20Object%20Reference))
  (if (Math|Boolean|Equal(Boolean) (and (.set Section) (Variables|/Game/Usinagem/Blueprints/BP_Configs_Gerais.BP_Configs_Gerais_C|GetPodeApertarReset (Variables|Default|GetRef_Configs_Gerais))) true)
    (Variables|Default|SetReset_Ligado true)
    (Default|LigarOGiroDasCastanhas (Variables|Default|GetRef_Avisos))
    (else
      (Variables|Default|SetReset_Ligado false)
      (if (Variables|/Game/Usinagem/Blueprints/BP_Configs_Gerais.BP_Configs_Gerais_C|GetEnergia (Variables|Default|GetRef_Configs_Gerais))
        (Default|AvisoProtecaoSolta (Variables|Default|GetRef_Avisos))
        (else
          (Default|ChaveGeral (Variables|Default|GetRef_Avisos)))))))

(event EventBeginPlay)

(event Collision|EventActorBeginOverlap
  (params (OtherActor :type Actor%20Object%20Reference)))

(event EventTick
  (params (DeltaSeconds :type Float%20%28single-precision%29)))

(fn ConstructionScript)