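; Emergency button for the machining scene, a draggable switch whose Ligado (on) state follows the section of its drag component.
; A looping half-second timer shows BP_Avisos warnings tagged "PortaLigada" with updated text while it is off, and targets them for hiding while on.
; Switching off also stops the sound of the referenced RefBotaoLigarCastanhas button.
; The K key flip-flops between both sections; a debug-print timer is never started.
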(event DragStateChangedSingle(Comp_Drag)
  (params (Identifier :type Name :default "None") (Section :type Struct%20Section%20Structure) (Source :type Actor%20Object%20Reference) (Pawn :type BP%20Pawn%20Base%20Object%20Reference))
  (bind _output_get (Variables|Default|SetLigado (.set Section)))
  (if (not _output_get)
    (Default|DesligarSom (Variables|Default|GetRef_BotaoLigar_Castanhas))))

(event Custom|Tagirandop
  (if (not (Variables|Default|GetLigado))
    (Development|PrintString "Botao de Emergencia Desligado" true true "(R=1.000000,G=0.000000,B=0.000000,A=1.000000)")))

(event Custom|CustomEvent
  (if (Variables|Default|GetLigado)
    (Rendering|SetActorHiddenInGame (stale _array_element) true)
    (else
      (bind _outactors (Actor|GetAllActorsOfClasswithTag "/Game/Usinagem/Blueprints/BP_Avisos.BP_Avisos_C" "PortaLigada"))
      (for _array_element _outactors
        (Rendering|Components|TextRender|SetText (Variables|/Game/Usinagem/Blueprints/BP_Avisos.BP_Avisos_C|GetAviso _array_element) (Variables|Default|GetValue))
        (Rendering|SetActorHiddenInGame _array_element false)))))

(event EventBeginPlay
  (Utilities|Time|SetTimerbyEvent (delegate Custom|CustomEvent) 0.5 true))

(event Collision|EventActorBeginOverlap
  (params (OtherActor :type Actor%20Object%20Reference)))

(event EventTick
  (params (DeltaSeconds :type Float%20%28single-precision%29)))

(event Input|KeyboardEvents|K
  (params (Key :type Key%20Structure :default "None"))
  (:Pressed
    (Utilities|FlowControl|FlipFlop
      (:A
        (Default|MovetoSection (Variables|Default|GetComp_Drag) "None" "Ligado"))
      (:B
        (Default|MovetoSection (Variables|Default|GetComp_Drag) "None" "Desligado")))))

(fn ConstructionScript)