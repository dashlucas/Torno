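; BP_Manivelairmaonovo is a Blueprint in the Usinagem (machining) content, named as a crank handle (manivela), that tracks drag input.
; Its Comp_Drag component's constant drag-state event copies distance, percent and velocity into Blueprint variables.
; A function named Teste stores three inputs and writes each to Procent in sequence, leaving the third as final; its other two inputs are unused.
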(event DragStateChangedConstant(Comp_Drag)
  (params (Name :type Name :default "None") (Distance :type Float%20%28single-precision%29) (Procent :type Float%20%28single-precision%29) (Velocity :type Float%20%28single-precision%29) (Source :type Actor%20Object%20Reference) (Pawn :type BP%20Pawn%20Base%20Object%20Reference))
  (Variables|Default|SetDistance Distance)
  (Variables|Default|SetProcent Procent)
  (Variables|Default|SetVelocity Velocity))

(fn ConstructionScript)

(fn Teste
  (params (m1 :type Float%20%28single-precision%29) (m2 :type Float%20%28single-precision%29) (m3 :type Float%20%28single-precision%29) (mp :type Float%20%28single-precision%29) (NewParam :type Actor%20Object%20Reference))
  (Variables|Default|SetM%201 m1)
  (Variables|Default|SetM%202 m2)
  (Variables|Default|SetM%203 m3)
  (Utilities|FlowControl|Sequence
    (:then_0
      (Variables|Default|SetProcent (Variables|Default|GetM%201)))
    (:then_1
      (Variables|Default|SetProcent (Variables|Default|GetM%202)))
    (:then_2
      (Variables|Default|SetProcent (Variables|Default|GetM%203)))))