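; BP_Avisos is a warning-message actor for the machining (Usinagem) content, showing timed notices about protection, main power, reset and chuck-jaw rotation.
; It starts hidden on BeginPlay.
; Each custom event unhides the actor, sets the Aviso text to its message, then hides it again after a fixed delay.
; The events are independent copies of this sequence, with no shared function or handling of overlapping messages.
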(event Custom|Aviso%20Protecao%20Certa
  (Rendering|SetActorHiddenInGame false)
  (Rendering|Components|TextRender|SetText (Variables|Default|GetAviso) (Variables|Default|Getprotecao2))
  (Utilities|FlowControl|Delay 5.0)
  (Rendering|SetActorHiddenInGame true))

(event Custom|Botao%20Castanhas%20Desativado
  (Rendering|SetActorHiddenInGame false)
  (Rendering|Components|TextRender|SetText (Variables|Default|GetAviso) (Variables|Default|GetLigarCastanhas2))
  (Utilities|FlowControl|Delay 5.0)
  (Rendering|SetActorHiddenInGame true))

(event Custom|Aviso%20Protecao%20Solta
  (Rendering|SetActorHiddenInGame false)
  (Rendering|Components|TextRender|SetText (Variables|Default|GetAviso) (Variables|Default|Getprotecao))
  (Utilities|FlowControl|Delay 5.0)
  (Rendering|SetActorHiddenInGame true))

(event Custom|Chave%20Geral
  (Rendering|SetActorHiddenInGame false)
  (Rendering|Components|TextRender|SetText (Variables|Default|GetAviso) (Variables|Default|GetEnergia%20Desligada-Ligada))
  (Utilities|FlowControl|Delay 5.0)
  (Rendering|SetActorHiddenInGame true))

(event Custom|Apertar%20Reset
  (Rendering|SetActorHiddenInGame false)
  (Rendering|Components|TextRender|SetText (Variables|Default|GetAviso) (Variables|Default|GetApertarReset))
  (Utilities|FlowControl|Delay 5.0)
  (Rendering|SetActorHiddenInGame true))

(event Custom|Ligar%20o%20Giro%20das%20castanhas
  (Rendering|SetActorHiddenInGame false)
  (Rendering|Components|TextRender|SetText (Variables|Default|GetAviso) (Variables|Default|GetLigarCastanhas))
  (Utilities|FlowControl|Delay 5.0)
  (Rendering|SetActorHiddenInGame true))

(event EventTick
  (params (DeltaSeconds :type Float%20%28single-precision%29)))

(event EventBeginPlay
  (Rendering|SetActorHiddenInGame true)
  (Utilities|FlowControl|Delay 0.2))

(fn ConstructionScript)