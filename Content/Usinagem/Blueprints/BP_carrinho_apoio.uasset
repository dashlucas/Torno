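; BP_carrinho_apoio is a machining support carriage that slides along X within a 31-unit travel range measured from its start location.
; Comp_Velocity's VelocityChanged event supplies the step, added as a local offset after direction checks against the range limits stored at BeginPlay.
; PosicaodasManivelas shifts three referenced crank handles by the same value in world X.
; Debug prints mark each branch.
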(event VelocityChanged(Comp_Velocity)
  (params (SourceInfo :type Struct%20Component%20Source%20Info%20Structure) (Value :type Struct%20Velocity%20Structure))
  ;[1 1 1] Setar a velocidade e seu multiplicador
  (Variables|Default|SetValue%20Velocity (/ (.velocity Value) 1.0))
  ;[1 1 1] Verificador de Posição final e inicial
  (if (>= (.x (Variables|Default|GetPosition%20carrinho%20inicial)) (.x (Variables|Default|GetPosition%20carrinho%20final)))
    ;[1 1 1] Verifica se está indo para a direita.
    (if (> (Variables|Default|GetValue%20Velocity) 0.0)
      ;[1 1 1] Verifica se a posição do carrinho está maior que o range
      (if (> (.x (Transformation|GetActorLocation)) (.x (Variables|Default|GetPosition%20carrinho%20inicial)))
        ;[1 1 1] Se a velocidade estiver positiva ele não anda, se estiver negativa ele anda
        (if (< (Variables|Default|GetValue%20Velocity) 0.0)
          (Transformation|AddActorLocalOffset (Math|Vector|MakeVector (Variables|Default|GetValue%20Velocity) 0.0 0.0) false false)
          (Development|PrintString "batata")
          (CallFunction|PosicaoDasManivelas))
        (else
          ;[1 1 1] Verificador de direção de movimento
          (if (< (Variables|Default|GetValue%20Velocity) 0.0)
            ;[1 1 1] Ele se movimenta para a esquerda
            (Transformation|AddActorLocalOffset (Math|Vector|MakeVector (Variables|Default|GetValue%20Velocity) 0.0 0.0) false false)
            (Development|PrintString "2")
            (CallFunction|PosicaoDasManivelas)
            (else
              ;[1 1 1] Ele se movimenta para a direita
              (Transformation|AddActorLocalOffset (Math|Vector|MakeVector (Variables|Default|GetValue%20Velocity) 0.0 0.0) false false)
              (Development|PrintString "hmmm")
              (CallFunction|PosicaoDasManivelas)))))
      (else
        ;[1 1 1] Verifica se está dentro do range mínimo
        (if (< (.x (Transformation|GetActorLocation)) (.x (Variables|Default|GetPosition%20carrinho%20final)))
          (Development|PrintString "Hello")
          ;[1 1 1] Verifica direção, se positiva ele anda, se negativa
          (if (> (Variables|Default|GetValue%20Velocity) 0.0)
            (Transformation|AddActorLocalOffset (Math|Vector|MakeVector (Variables|Default|GetValue%20Velocity) 0.0 0.0) false false)
            (Development|PrintString "1")
            (CallFunction|PosicaoDasManivelas))
          (elif (< (Variables|Default|GetValue%20Velocity) 0.0)
            (Transformation|AddActorLocalOffset (Math|Vector|MakeVector (Variables|Default|GetValue%20Velocity) 0.0 0.0) false false)
            (Development|PrintString "sei la")
            (CallFunction|PosicaoDasManivelas)
            (else
              (Development|PrintString "hello 2")
              (CallFunction|PosicaoDasManivelas))))))
    (else
      ;[1 1 1] Não sei
      (Transformation|AddActorLocalOffset (Math|Vector|MakeVector (Variables|Default|GetValue%20Velocity) 0.0 0.0) false false)
      (Development|PrintString "caralho")
      (CallFunction|PosicaoDasManivelas))))

(event Custom|Posicao%20das%20Manivelas
  ;[1 1 1] Posicao das Manivelas
  (Transformation|AddActorWorldOffset (Variables|Referencias|GetRef_Manivelas) (Math|Vector|MakeVector (Variables|Default|GetValue%20Velocity) 0.0 0.0))
  (Development|PrintString "manivela"))

(event EventBeginPlay
  ;[1 1 1] Setar posição inicial e final
  (bind _output_get (Variables|Default|SetPosition%20carrinho%20inicial (Transformation|GetActorLocation)))
  (Variables|Default|SetPosition%20carrinho%20final (+ _output_get "-31.000000, 0, 0")))

(fn ConstructionScript)