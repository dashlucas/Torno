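; Speed control button for the machining scene that turns drag input into rotation of the referenced chuck jaws (Castanhas).
; While dragged, it stores distance, percent and velocity, then passes the percent to the general config's ComVelocidades to get a rotation value.
; When the latch reports a release, it adds that stored rotation to the jaws' root component as a relative rotation.
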(event DragStateChangedConstant(Comp_Drag)
  (params (Name :type Name :default "None") (Distance :type Float%20%28single-precision%29) (Procent :type Float%20%28single-precision%29) (Velocity :type Float%20%28single-precision%29) (Source :type Actor%20Object%20Reference) (Pawn :type BP%20Pawn%20Base%20Object%20Reference))
  (Variables|Default|SetDistance Distance)
  (Variables|Default|SetProcent Procent)
  (Variables|Default|SetVelocity Velocity)
  (bind _rotation (Default|ComVelocidades (Variables|Default|GetRef_Configs_Gerais) 0.0 (Variables|Default|GetProcent) 0.0 self))
  (Variables|Default|SetRotation _rotation))

(event LatchActorLatchReleased(Comp_Latch_Drag)
  (params (ReleasingPawn :type BP%20Pawn%20Base%20Object%20Reference) (ReleasingActor :type Actor%20Object%20Reference))
  (Transformation|AddRelativeRotation (Variables|/Script/Engine.Actor|GetRootComponent (Variables|Default|GetRef_castanhas)) (Variables|Default|GetRotation) false false))

(event EventBeginPlay)

(event Collision|EventActorBeginOverlap
  (params (OtherActor :type Actor%20Object%20Reference)))

(event EventTick
  (params (DeltaSeconds :type Float%20%28single-precision%29)))

(fn ConstructionScript)