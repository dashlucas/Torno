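; General controller for a machining simulator that links the machine's power indicator, safety interlocks and hand cranks.
; The power trigger toggles the indicator sphere's material and the machine-on flag.
; The protection trigger checks chuck guard, window guard and emergency button, but only prints whether startup is allowed.
; Cranks 2 and 3 lerp the carriage along X by turn percentage; crank 1 and the latch/release functions are stubs.
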(event ComponentTriggered(Comp_Trigger_Protecao)
  (params (SourceInfo :type Struct%20Component%20Source%20Info%20Structure) (Name :type Name :default "None"))
  (CallFunction|PodeLigar (Variables|/Game/Usinagem/Blueprints/BP_protecao_1.BP_protecao_1_C|GetFechado (Variables|Referencias|GetRef_Pretecao_Castanhas)) (Variables|/Game/Usinagem/Blueprints/BP_vidro_janela.BP_vidro_janela_C|GetFechado (Variables|Referencias|GetRef_Protecao_Janela)) (Variables|/Game/Usinagem/Blueprints/BP_BotaoEmergencia.BP_BotaoEmergencia_C|GetLigado (Variables|Referencias|GetRef_Botao_Emergencia)) 0.0))

(event ComponentTriggered(Comp_Trigger_Energia)
  (params (SourceInfo :type Struct%20Component%20Source%20Info%20Structure) (Name :type Name :default "None"))
  (bind _ref_esfera_ligar (Variables|Referencias|GetRef_Esfera_Ligar))
  (bind _staticmeshcomponent (Variables|/Script/Engine.StaticMeshActor|GetStaticMeshComponent _ref_esfera_ligar))
  (if (Utilities|Name|Equal(Name) Name "On")
    (Rendering|Material|SetMaterial _staticmeshcomponent 0 "/Game/Usinagem/Materials/MI_Luz_Maquina_Ligada.MI_Luz_Maquina_Ligada")
    (Variables|Default|SetMaquina_Ligada true)
    (else
      (Rendering|Material|SetMaterial _staticmeshcomponent 0 "/Game/Usinagem/Materials/M_Plastic.M_Plastic")
      (Variables|Default|SetMaquina_Ligada false))))

(event EventBeginPlay)

(fn ConstructionScript)

(fn ComManivelas
  (params (Velocity :type Float%20%28single-precision%29) (Percent :type Float%20%28single-precision%29) (Distance :type Float%20%28single-precision%29) (Actor :type Actor%20Object%20Reference))
  (Variables|Default|SetPercent Percent)
  (Utilities|FlowControl|Sequence
    (:then_0
      (if (== Actor (Variables|Referencias|GetRef_BP_Manivela_1))
        (if true
          _)))
    (:then_1
      (if (== Actor (Variables|Referencias|GetRef_BP_Manivela_2))
        (Transformation|SetActorLocation (Variables|Referencias|GetRef_BP_Carrinho) (Math|Vector|MakeVector (Math|Float|Lerp 164.0 203.0 (Variables|Default|GetPercent)) 87.849236 164.582886) false false)
        (Variables|Default|SetDistancia%20On%20Latch_0 0.0)
        (Development|PrintString (Utilities|String|Append "Distancia Porcent" (Utilities|String|ToString(Float) (Variables|Default|GetPercent)) "       Distancia On Latch 0" (Utilities|String|ToString(Float) (Variables|Default|GetDistancia%20On%20Latch_0)) "       Distancia Atual" (Utilities|String|ToString(Float) (Variables|Default|GetDistance%20Atual))) true true "(R=0.000000,G=0.660000,B=1.000000,A=1.000000)" 1e+01)
        (return (Variables|Default|GetDistancia%20On%20Latch))))
    (:then_2
      (if (== Actor (Variables|Referencias|GetRef_BP_Manivela_3))
        (Transformation|SetActorLocation (Variables|Referencias|GetRef_BP_Carrinho) (Math|Vector|MakeVector (Math|Float|Lerp 164.0 203.0 (Variables|Default|GetPercent)) 87.849236 164.582886) false false)
        (Variables|Default|SetDistancia%20On%20Latch_1 0.0)))))

(fn GotLatched
  (params (Distancia%20on%20latch :type Float%20%28single-precision%29) (Distancia%20on%20released :type Float%20%28single-precision%29) (Disctancia%20atual :type Float%20%28single-precision%29) (Actor :type Actor%20Object%20Reference)))

(fn OnReleased
  (params (Distancia%20on%20latch :type Float%20%28single-precision%29) (Distancia%20on%20released :type Float%20%28single-precision%29) (Porcent :type Float%20%28single-precision%29)))

(fn PodeLigar
  (params (Protecao%20Castanhas :type Boolean) (Protecao%20Janela :type Boolean) (Botao%20Emergencia :type Boolean) (NewParam3 :type Float%20%28single-precision%29))
  (if (Math|Boolean|ANDBoolean Protecao%20Castanhas Protecao%20Janela Botao%20Emergencia)
    (Development|PrintString "PODE LIGAR")
    (else
      (Development|PrintString "Desliga"))))