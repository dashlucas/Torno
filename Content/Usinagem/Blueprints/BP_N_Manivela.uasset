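; BP_N_Manivela is a crank handle actor in the machining content that spins in response to velocity changes.
; Its Comp_Velocity component's VelocityChanged event scales the velocity down and adds it as a local roll rotation, stepping once per event rather than on Tick.
; An unconnected ComManivelas call on RefConfigsGerais never runs, and BeginPlay is empty.
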(event VelocityChanged(Comp_Velocity)
  (params (SourceInfo :type Struct%20Component%20Source%20Info%20Structure) (Value :type Struct%20Velocity%20Structure))
  (bind _output_get (Variables|Default|SetValue%20Velocity (/ (.velocity Value) 1e+02)))
  (Transformation|AddActorLocalRotation (Math|Rotator|MakeRotator _output_get 0.0 0.0) false false))

(event EventBeginPlay)

(event Collision|EventActorBeginOverlap
  (params (OtherActor :type Actor%20Object%20Reference)))

(fn ConstructionScript)