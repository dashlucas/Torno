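; BP_apoio_castanhas is a rotating support actor ("apoio castanhas", chestnut support) driven by a linked on/off button.
; Each tick, while the button's TaGirando is true, it rotates its static mesh by the referenced speed object's Rotation.
; Otherwise the AtéZero timeline scales that rotation via LerpRotator, intended as a spin-down, and prints it for debugging.
; The timeline calls PlayFromStart every tick, so it keeps restarting.
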(event EventBeginPlay
  (Transformation|AddRelativeRotation (Variables|Debug|GetStaticMeshComponent) "0, 0, 0" false false))

(event Collision|EventActorBeginOverlap
  (params (OtherActor :type Actor%20Object%20Reference)))

(event EventTick
  (params (DeltaSeconds :type Float%20%28single-precision%29))
  (if (Variables|/Game/Usinagem/Blueprints/BP_BotaoLigar_Castanhas.BP_BotaoLigar_Castanhas_C|GetTa_girando (Variables|Default|GetRef_Botao_Ligar_Castanhas))
    (Transformation|AddRelativeRotation (Variables|Debug|GetStaticMeshComponent) (Variables|/Game/Usinagem/Blueprints/BP_Botao_Velocidade.BP_Botao_Velocidade_C|GetRotation (Variables|Default|GetRef_Velocidade)) false false)
    (else
      (bind _zerando (Timeline|Até%20Zero PlayFromStart)
        (:Update
          (Transformation|AddRelativeRotation (Variables|Debug|GetStaticMeshComponent) (Math|Rotator|Lerp(Rotator) "0, 0, 0" (Variables|/Game/Usinagem/Blueprints/BP_Botao_Velocidade.BP_Botao_Velocidade_C|GetRotation (Variables|Default|GetRef_Velocidade)) _zerando) false false)
          (Development|PrintString (Utilities|String|ToString(Rotator) (Math|Rotator|Lerp(Rotator) "0, 0, 0" (Variables|/Game/Usinagem/Blueprints/BP_Botao_Velocidade.BP_Botao_Velocidade_C|GetRotation (Variables|Default|GetRef_Velocidade)) _zerando)) true true "(R=0.000000,G=1.000000,B=0.040708,A=1.000000)"))))))

(fn ConstructionScript)